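; Player character Blueprint that handles movement, looking, jumping and interaction with objects in the world.
; Axis inputs feed movement along the actor's forward and right vectors and drive controller yaw and pitch.
; Pressing E line-traces for PhysicsBody objects from the actor's location along its forward vector, not the camera's view, with debug drawing on.
; A hit sends InteractMessage to the struck actor.
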(event `Key|E`
  (params (Key :type "Key Structure"))
  (bind _returnvalue (`ActorComponent.GetOwner` (`self.Camera`)))
  (bind _returnvalue_2 (`self.K2_GetActorLocation` _returnvalue))
  ;[1 1 1] press button
  (:`Pressed`
    (bind (_outhit _returnvalue_3) (`KismetSystemLibrary.LineTraceSingleForObjects` :`Start` _returnvalue_2 :`End` (+ _returnvalue_2 (* (`self.GetActorForwardVector` _returnvalue) 500.0)) :`ObjectTypes` (`|MakeArray` "ObjectTypeQuery4" :!type "EObjectTypeQuery Enum") :`DrawDebugType` "ForDuration"))
    (if _returnvalue_3
      (message `/Game/BluePrints/BP_button/BP_communication.Interact` (`.HitActor` (`GameplayStatics.BreakHitResult` _outhit))))))

(event `InputAxis|MoveForward`
  (params (AxisValue :type "Float (single-precision)"))
  ;[1 1 1] movement
  (`self.AddMovementInput` (`self.GetActorForwardVector`) AxisValue))

(event `InputAxis|MoveRight`
  (params (AxisValue :type "Float (single-precision)"))
  ;[1 1 1] movement
  (`self.AddMovementInput` (`self.GetActorRightVector`) AxisValue))

(event `InputAction|Jump`
  (params (Key :type "Key Structure"))
  ;[1 1 1] movement
  (:`Pressed`
    (`self.Jump`)))

(event `InputAxis|LookUp`
  (params (AxisValue :type "Float (single-precision)"))
  ;[1 1 1] overview
  (`self.AddControllerPitchInput` AxisValue))

(event `InputAxis|Turn`
  (params (AxisValue :type "Float (single-precision)"))
  ;[1 1 1] overview
  (`self.AddControllerYawInput` AxisValue))

(fn `UserConstructionScript`)