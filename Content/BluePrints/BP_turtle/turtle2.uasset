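; Turtle pawn Blueprint that starts AI-driven movement toward an actor once it is possessed.
; On possession it adds a FloatingPawnMovement component at runtime, then uses short delays to stop the AI controller's movement and issue a MoveToActor.
; BeginPlay, overlap and Tick are disabled placeholders, and the construction script only calls its parent.
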(event `self.ReceivePossessed`
  (params (NewController :type "Controller Object Reference"))
  (bind _aicontr (`self.aicontr`))
  (`AddComponent|NODE_AddFloatingPawnMovement-0`)
  (`KismetSystemLibrary.Delay` 1.0)
  (`Controller.StopMovement` _aicontr)
  (`KismetSystemLibrary.Delay` 0.5)
  (`AIController.MoveToActor` _aicontr null -1.0 true true true null true))

(fn `UserConstructionScript`
  (`parent.UserConstructionScript`))