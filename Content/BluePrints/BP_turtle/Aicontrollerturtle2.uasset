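; AI controller for a turtle pawn that plays an explosion effect and sound on possession, then walks it to a TargetPoint.
; The target is the second TargetPoint returned by GetAllActorsOfClass.
; A delay loop repeatedly stops movement and reissues AIMoveTo, producing stop-and-go motion.
; On arrival it spawns sparks with a timed sound and destroys the pawn.
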(event `self.ReceivePossess`
  (params (PossessedPawn :type "Pawn Object Reference"))
  (bind _returnvalue (`self.K2_GetActorLocation` PossessedPawn))
  (bind _returnvalue_2 (`self.K2_GetActorLocation` PossessedPawn))
  (`GameplayStatics.SpawnEmitterAtLocation` "/Game/StarterContent/Particles/P_Explosion.P_Explosion" _returnvalue_2)
  (`GameplayStatics.SpawnSoundAtLocation` "/Game/StarterContent/Audio/Explosion01.Explosion01" _returnvalue_2 (struct) 1.0 1.0 0.0 null null)
  (bind _outactors (`GameplayStatics.GetAllActorsOfClass` "/Script/Engine.TargetPoint"))
  (`|AIMoveTo` PossessedPawn (0.0 0.0 0.0) (`|GetArrayItem` _outactors 1) :!label _label
    (:`then`
      (`KismetSystemLibrary.Delay` 1.0)
      (`self.StopMovement`)
      (`KismetSystemLibrary.Delay` 0.5)
      (goto _label))
    (:`OnSuccess`
      (`GameplayStatics.SpawnEmitterAtLocation` "/Game/VFX/P_Sparks.P_Sparks" _returnvalue)
      (bind _returnvalue_3 (`GameplayStatics.SpawnSoundAtLocation` "/Game/StarterContent/Audio/Fire_Sparks01.Fire_Sparks01" _returnvalue (struct) 1.0 1.0 0.0 null null))
      (`AudioComponent.StopDelayed` _returnvalue_3 5.0)
      (`self.K2_DestroyActor` PossessedPawn))))

(fn `go`)

(fn `sectick`)

(fn `UserConstructionScript`)